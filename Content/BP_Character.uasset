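; Character Blueprint that puts the HUD on screen and handles health, damage feedback and game over.
; BeginPlay creates the MyHUD widget and adds it to the viewport.
; AnyDamage subtracts Health through a DoOnce gate, which stays closed while ShowDamageTint pulses and a short delay follows, ignoring further hits during that window.
; When Health reaches zero or below, EventGameOver quits the game outright.
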(event Custom|EventGameOver
  (Game|QuitGame 0 "Quit" false))

(event EventBeginPlay
  ;[1 1 1] Establish connection to the HUD
  (bind _returnvalue (UserInterface|CreateWidget "/Game/MyHUD.MyHUD_C"))
  (UserInterface|Viewport|AddtoViewport _returnvalue 0))

(event Collision|EventActorBeginOverlap
  (params (OtherActor :type Actor%20Object%20Reference)))

(event EventTick
  (params (DeltaSeconds :type Float%20%28single-precision%29)))

(event Game|Damage|EventAnyDamage
  (params (Damage :type Float%20%28single-precision%29) (DamageType :type Damage%20Type%20Object%20Reference) (InstigatedBy :type Controller%20Object%20Reference) (DamageCauser :type Actor%20Object%20Reference))
  ;[1 1 1] Damage Logic
  (Utilities|FlowControl|DoOnce false :!label _label
    (:Completed
      (bind _output_get (Variables|Default|SetHealth (- (Variables|Default|GetHealth) Damage)))
      (if (<= _output_get 0.0)
        (CallFunction|EventGameOver)
        (else
          (Variables|Default|SetShowDamageTint true)
          (Utilities|FlowControl|Delay 0.3)
          (Variables|Default|SetShowDamageTint false)
          (Utilities|FlowControl|Delay 0.2)
          (goto _label Reset))))))

(fn ConstructionScript)