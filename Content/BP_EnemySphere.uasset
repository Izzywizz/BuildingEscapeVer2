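; BP_EnemySphere is an enemy hazard that moves around its starting location and damages BP_Character on overlap.
; On BeginPlay it stores that location and plays a timeline, adding either the X or Y movement track as an offset, chosen by UseXMovement.
; Movement sets the location without sweeping, and each begin-overlap with the character applies a small fixed amount of damage.
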(event EventBeginPlay
  (bind _output_get (Variables|Default|SetInitialEnemyLocation (Transformation|GetActorLocation)))
  (bind (_direction _xmovementtrack _ymovementtrack) (Timeline|EnemySphereTimeline Play)
    (:Update
      (if (Variables|Default|GetUseXMovement)
        (Transformation|SetActorLocation (+ _output_get _xmovementtrack) false false)
        (else
          (Transformation|SetActorLocation (+ _output_get _ymovementtrack) false false))))))

(event Collision|EventActorBeginOverlap
  (params (OtherActor :type Actor%20Object%20Reference))
  (bind _asbp_character (Utilities|Casting|CastToBP_Character OtherActor))
  (Game|Damage|ApplyDamage _asbp_character 0.2 0 0))

(event EventTick
  (params (DeltaSeconds :type Float%20%28single-precision%29)))

(fn ConstructionScript)